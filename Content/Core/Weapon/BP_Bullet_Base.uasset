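; BP_Bullet_Base is a base bullet actor for weapons that damages zombie NPCs on impact.
; Its sphere collision hit event sends BP_NPC_Zombie hits through DamageZombie, which applies damage credited to the first player controller, prints debug text, then destroys the bullet.
; BP_Wall hits only destroy it, while other actors trigger nothing.
; GetDamage exposes the damage value.
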(event `self.Sphere collision.OnComponentHit`
  (params (HitComponent :type "PrimitiveComponent Object Reference") (OtherActor :type "Actor Object Reference") (OtherComp :type "PrimitiveComponent Object Reference") (NormalImpulse :type "Vector Structure") (Hit :type "HitResult Structure (by ref)"))
  (`|ExecutionSequence`
    (:`then_0`
      (bind _asbp_npc_zombie (cast `/Game/Character/NPC/BP_NPC_Zombie` OtherActor))
      (`GameplayStatics.ApplyDamage` _asbp_npc_zombie (`self.Damage`) (`GameplayStatics.GetPlayerController` 0) self "/Script/Engine.DamageType")
      (`KismetSystemLibrary.PrintText` "Hitted Zombie")
      (`self.K2_DestroyActor`))
    (:`then_1`
      (cast `/Game/SceneObjects/BP_Wall` OtherActor)
      (`self.K2_DestroyActor`))))

(fn `GetDamage`
  (returns (Damage :type "Float (double-precision)"))
  (return (`self.Damage`)))

(fn `UserConstructionScript`)