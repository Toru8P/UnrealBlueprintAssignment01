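; Base weapon Blueprint that handles projectile firing, magazine and reserve ammo, and reloading.
; Shoot spends a loaded round to spawn the projectile and muzzle effect at GetShootSpot, with a retriggerable delay gating fire rate.
; Reload fills the magazine from reserve; AddReserveAmmo clamps reserve and auto-reloads when both pools were empty.
; GetShootSpot raises a script error as a placeholder for child overrides; getters expose ammo and weapon type.
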(event `/Game/Core/Weapon/I_Weapon.AddReserveAmmo`
  (params (Amount :type Integer))
  ;[0.1179 0 0.15 0.5] Reserve Ammo Logic
  (set `self.ReserveAmmo` (`KismetMathLibrary.Min` (`KismetMathLibrary.Max` 0 (+ Amount (`self.ReserveAmmo`))) (`self.MaxReserveAmmo`)))
  (if (and (== Amount (`self.ReserveAmmo`)) (== (`self.LoadedBullets`) 0))
    (`/Game/Core/Weapon/I_Weapon.Reload`)))

(event `/Game/Core/Weapon/I_Weapon.Shoot`
  (bind _loadedbullets (`self.LoadedBullets`))
  ; Shoot
  (if (`self.CanShoot`)
    (`|ExecutionSequence`
      (:`then_0`
        (set `self.CanShoot` false)
        (if (> _loadedbullets 0)
          (bind _result (`/Engine/EditorBlueprintResources/StandardMacros.DecrementInt` _loadedbullets)
            (:`  `
              (set `self.LoadedBullets` _result)
              (bind _shootspot (`self.GetShootSpot`))
              (`|SpawnActorFromClass` (`self.ProjectileClass`) _shootspot "AlwaysSpawn" "MultiplyWithRoot" null null)
              (`GameplayStatics.SpawnEmitterAtLocation` "/Game/Core/Particle/CPS_Shoot.CPS_Shoot" (.location _shootspot) (struct) (0.3 0.3 0.3))
              (`KismetSystemLibrary.PrintText` (`|FormatText` "Currently reserved: {ReservedAmmo} - Currently loaded: {LoadedAmmo}" (`self.ReserveAmmo`) (`self.LoadedBullets`)))))
          (else
            (`KismetSystemLibrary.PrintText` "You have no bullets!"))))
      (:`then_1`
        (`KismetSystemLibrary.RetriggerableDelay` (`self.FireRate`))
        (set `self.CanShoot` true)))))

(event `/Game/Core/Weapon/I_Weapon.Reload`
  ; Reload
  ;;[0.1184 0.15 0 0.5] Check if reload is needed
  (if (<= (`self.ReserveAmmo`) 0)
    _
    (elif (not (== (`self.LoadedBullets`) (`self.MagazineSize`)))
      (bind _returnvalue (`self.GetRequiredAmountOnReload`))
      (if (> _returnvalue (`self.ReserveAmmo`))
        (set `self.LoadedBullets` (+ (`self.ReserveAmmo`) (`self.LoadedBullets`)))
        (set `self.ReserveAmmo` 0)
        (else
          (set `self.LoadedBullets` (`self.MagazineSize`))
          (set `self.ReserveAmmo` (- (`self.ReserveAmmo`) _returnvalue)))))))

(fn `GetLoadedBullets`
  (returns (Amount :type Integer))
  (return (`self.LoadedBullets`)))

(fn `GetRequiredAmountOnReload`
  (returns (ReturnValue :type Integer))
  (return (- (`self.MagazineSize`) (`self.LoadedBullets`))))

(fn `GetReserveAmmo`
  (returns (ReserveSize :type Integer))
  (return (`self.ReserveAmmo`)))

(fn `GetShootSpot`
  (returns (ShootSpot :type "Transform Structure"))
  (`KismetSystemLibrary.RaiseScriptError` "Shoot Spot wasnt implemented")
  (return))

(fn `GetWeaponType`
  (returns (WeaponType :type "/Game/Core/Weapon/E_WeaponType Enum"))
  (return (`self.WeaponType`)))

(fn `UserConstructionScript`)