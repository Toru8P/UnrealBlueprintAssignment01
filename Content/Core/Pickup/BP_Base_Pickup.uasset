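; Base pickup actor that spins, bobs and triggers pickup logic when the player character overlaps its box.
; If CanPickup is set, the overlap passes the cast BP_PlayerCharacter to HandlePickup, which child classes must override because the base raises a script error.
; Tick animates it in code, applying yaw rotation and adding a sine-plus-HeightOffset term to the current Z each frame.
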(event `self.Box.OnComponentBeginOverlap`
  (params (OverlappedComponent :type "PrimitiveComponent Object Reference") (OtherActor :type "Actor Object Reference") (OtherComp :type "PrimitiveComponent Object Reference") (OtherBodyIndex :type Integer) (bFromSweep :type Boolean) (SweepResult :type "HitResult Structure (by ref)"))
  (bind _returnvalue (`GameplayStatics.GetPlayerCharacter` 0))
  ;[0.1391 0.04545 0.15 0.5] Pickup Logic
  (if (== _returnvalue OtherActor)
    (if (`self.bCanPickup`)
      (bind _asbp_player_character (cast `/Game/Character/Player/BP_PlayerCharacter` _returnvalue))
      (`self.HandlePickup` _asbp_player_character)
      (else
        (`KismetSystemLibrary.PrintText` "Cant pickup")))))

(event `self.ReceiveTick`
  (params (DeltaSeconds :type "Float (single-precision)"))
  (bind (_returnvalue_x _returnvalue_y _returnvalue_z) (`KismetMathLibrary.BreakVector` (`self.K2_GetActorLocation`)))
  ; Pickup Rotation
  (`self.K2_AddActorLocalRotation` (`KismetMathLibrary.MakeRotator` 0.0 0.0 (* DeltaSeconds (`self.rotationSpeed`))))
  ; Floating Animation - Did it without animation graph
  (`self.K2_SetActorLocation` (`KismetMathLibrary.MakeVector` _returnvalue_x _returnvalue_y (+ (+ (* (`KismetMathLibrary.Sin` (* (`self.frequency `) (`KismetSystemLibrary.GetGameTimeInSeconds`))) (`self.amplitude`)) (`self.heightOffset`)) _returnvalue_z))))

(fn `HandlePickup`
  (params (`Player Ref` :type "/Game/Character/Player/BP_PlayerCharacter Object Reference"))
  (`KismetSystemLibrary.RaiseScriptError` "Handle Pickup Not Implemented"))

(fn `UserConstructionScript`)