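; Base gun pickup that offers a weapon to the player who collects it.
; HandlePickup tries to add WeaponRef to the player's inventory.
; Only when that add returns false does it grant the pickup's Ammo for that weapon and destroy itself; a successful add triggers no further action here.
; The event graph holds only disabled default events.
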(fn `HandlePickup`
  (params (`Player Ref` :type "/Game/Character/Player/BP_PlayerCharacter Object Reference"))
  (bind _weaponref (`self.weaponRef`))
  (bind _haveweapon (`/Game/Character/Player/BP_PlayerCharacter.AddWeaponToInventary` `Player Ref` _weaponref))
  (if (not _haveweapon)
    (`/Game/Character/Player/BP_PlayerCharacter.AddAmmoToInventary` `Player Ref` _weaponref (`self.ammo`))
    (`self.K2_DestroyActor`)))

(fn `UserConstructionScript`
  (`parent.UserConstructionScript`))